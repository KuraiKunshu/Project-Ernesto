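; Event-action actor that changes levels when it receives an Action event, using the message string as the level name.
; Action shows a BPW_ChangeScene widget, plays it, waits a delay scaled by play rate, then opens the level if the message is non-empty.
; BeginPlay prints a warning for listed actors lacking BPI_EventAction.
; Logic to forward messages to those actors and self-destroy is present but never runs.
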(event `self.ReceiveBeginPlay`
  (for _array_element _
    (if (not (`KismetSystemLibrary.DoesImplementInterface` (break `/Game/Kurai_Workspace/S_TriggerTemp` _array_element) "/Game/Kurai_Workspace/BlueprintTrigger/BPI_EventAction.BPI_EventAction_C"))
      (`KismetSystemLibrary.PrintString` (`KismetStringLibrary.Concat_StrStr` "NO ACTION INTERFACE ON " (`KismetSystemLibrary.GetDisplayName` (break `/Game/Kurai_Workspace/S_TriggerTemp` _array_element)))))))

(event `self.Action`
  (params (`Action Type` :type "/Game/Kurai_Workspace/BlueprintTrigger/E_ActionType Enum" :default "NewEnumerator1") (msg :type String))
  (bind _play_rate (`self.Play Rate`))
  (bind _returnvalue (`|CreateWidget` "/Game/Kurai_Workspace/BPW_ChangeScene.BPW_ChangeScene_C" (`GameplayStatics.GetPlayerController` 0)))
  (`UserWidget.AddToViewport` _returnvalue 0)
  (`/Game/Kurai_Workspace/BPW_ChangeScene.Play` _returnvalue (`self.Play Mode`) _play_rate)
  (`KismetSystemLibrary.Delay` (/ 2.0 _play_rate))
  (if (not (`KismetStringLibrary.EqualEqual_StrStr` msg))
    (`GameplayStatics.OpenLevel` (`KismetStringLibrary.Conv_StringToName` msg))))

(fn `UserConstructionScript`)