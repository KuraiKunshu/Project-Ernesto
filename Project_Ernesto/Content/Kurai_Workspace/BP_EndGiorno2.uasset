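; BP_EndGiorno2 is a trigger actor, apparently for the end of day two, that starts a dialogue with Zio on sphere overlap.
; When ActorTrigger, defaulting to the player pawn, enters, it assigns Zio's BPC_DialogueSystem to the first-person character and calls InteractMessage.
; BeginPlay prints warnings for ToTrigger actors lacking BPI_EventAction, but those actors are never triggered here and Action is empty.
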(event `self.ReceiveBeginPlay`
  (`|ExecutionSequence`
    (:`then_0`
      (for _array_element (`self.ToTrigger`)
        (if (not (`KismetSystemLibrary.DoesImplementInterface` (break `/Game/Kurai_Workspace/S_TriggerTemp` _array_element) "/Game/Kurai_Workspace/BlueprintTrigger/BPI_EventAction.BPI_EventAction_C"))
          (`KismetSystemLibrary.PrintString` (`KismetStringLibrary.Concat_StrStr` "NO ACTION INTERFACE ON " (`KismetSystemLibrary.GetDisplayName` (break `/Game/Kurai_Workspace/S_TriggerTemp` _array_element)))))))
    (:`then_1`
      (`/Engine/EditorBlueprintResources/StandardMacros.IsValid` (`self.Actor Trigger`)
        (:`Is Not Valid`
          (set `self.Actor Trigger` (`GameplayStatics.GetPlayerPawn` 0)))))))

(event `self.Sphere.OnComponentBeginOverlap`
  (params (OverlappedComponent :type "PrimitiveComponent Object Reference") (OtherActor :type "Actor Object Reference") (OtherComp :type "PrimitiveComponent Object Reference") (OtherBodyIndex :type Integer) (bFromSweep :type Boolean) (SweepResult :type "HitResult Structure (by ref)"))
  (if (== OtherActor (`self.Actor Trigger`))
    (bind _asbp_first_person_character (cast `/Game/FirstPerson/Blueprints/BP_FirstPersonCharacter` (`GameplayStatics.GetPlayerPawn` 0)))
    (bind _output_get (set `/Game/FirstPerson/Blueprints/BP_FirstPersonCharacter.Dialogue Comp ref` (`self.GetComponentByClass` (`self.zio`) "/Game/Kurai_Workspace/DialogSystem/BPC_DialogueSystem.BPC_DialogueSystem_C") _asbp_first_person_character))
    (message `/Game/Kurai_Workspace/Enemy/Blueprints/Interfaces/IInteractable.Interact` _output_get)))

(event `self.Action`
  (params (`Action Type` :type "/Game/Kurai_Workspace/BlueprintTrigger/E_ActionType Enum" :default "NewEnumerator1") (msg :type String)))

(fn `UserConstructionScript`)