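; BP_EventManager is an event manager that configures trigger actors from per-day event data.
; On BeginPlay it calls LinkComponent for day 0, which looks that day up in the DailyEvents map.
; For each listed event, it copies the actors to trigger, action type and message into the BPC_TriggerComponent of the assigned actor.
; The graph also holds leftover unconnected test nodes for printing and string conversion.
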(event `self.ReceiveBeginPlay`
  (`self.Link Component` 0))

(event `Link Component`
  (params (`Day Number` :type Integer))
  (bind (_value _returnvalue) (`BlueprintMapLibrary.Map_Find` (`self.DailyEvents`) `Day Number`))
  (if _returnvalue
    (for _array_element (break `/Game/Kurai_Workspace/BlueprintTrigger/S_DailyEvents` _value)
      (bind _returnvalue_2 (`self.GetComponentByClass` (break `/Game/Kurai_Workspace/BlueprintTrigger/S_EventTrigger` _array_element) "/Game/Kurai_Workspace/BlueprintTrigger/BPC_TriggerComponent.BPC_TriggerComponent_C"))
      (set `/Game/Kurai_Workspace/BlueprintTrigger/BPC_TriggerComponent.Actors to Instigate` (`.ActorstoTrigger_31_186A203E45777A0D39912492F1D2396E` (break `/Game/Kurai_Workspace/BlueprintTrigger/S_EventTrigger` _array_element)) _returnvalue_2)
      (set `/Game/Kurai_Workspace/BlueprintTrigger/BPC_TriggerComponent.Action Type` (`.ActionType_35_8EEF12F34B105CA915316BB93374D845` (break `/Game/Kurai_Workspace/BlueprintTrigger/S_EventTrigger` _array_element)) _returnvalue_2)
      (set `/Game/Kurai_Workspace/BlueprintTrigger/BPC_TriggerComponent.Msg` (`.msg_37_0BB3CE2B45D4C64446E9AAABFFF98650` (break `/Game/Kurai_Workspace/BlueprintTrigger/S_EventTrigger` _array_element)) _returnvalue_2))))

(fn `UserConstructionScript`)