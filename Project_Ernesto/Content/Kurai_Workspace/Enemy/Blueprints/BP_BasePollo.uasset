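; BP_BasePollo is a base Blueprint in the Enemy folder for a "Pollo" pawn that wanders on its own.
; On BeginPlay it runs the parent logic, sets a random uniform scale, and starts a looping timer with a varied initial delay.
; Each timer tick sends it by AI Move To toward a random reachable navmesh point within a radius of its current location.
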(event `self.ReceiveBeginPlay`
  (`parent.ReceiveBeginPlay`)
  (`self.SetActorScale3D` (`KismetMathLibrary.Conv_DoubleToVector` (`KismetMathLibrary.RandomFloatInRange` 0.4 1.0)))
  (`KismetSystemLibrary.K2_SetTimerDelegate` (delegate `Move Within Range`) 15.0 true false 0.0 8.0))

(event `Move Within Range`
  (`|AIMoveTo` self (`NavigationSystemV1.K2_GetRandomReachablePointInRadius` (`self.K2_GetActorLocation`) 1000.0 (`self.Nav Data`) null) null))

(fn `UserConstructionScript`
  (`parent.UserConstructionScript`))