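; BP_Pollo is a non-fighting "Pollo" entity that transforms into an alien monster when it receives a specific action.
; On BeginPlay it spawns passive and kills its referenced alien after a delay.
; The action plays transformation VFX and sound, kills the Pollo, then respawns the alien passive at its position.
; A timeline, its length set by the message, scales the alien mesh, then a scream montage leads into enabling combat.
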(event `self.ReceiveBeginPlay`
  (`parent.ReceiveBeginPlay`)
  (`self.Spawn` false "Player")
  (`/Engine/EditorBlueprintResources/StandardMacros.IsValid` (`self.Alien Ref`)
    (:`Is Valid`
      (`KismetSystemLibrary.Delay` 5.0)
      (`self.Death` (`self.Alien Ref`)))))

(event `/Game/Kurai_Workspace/BlueprintTrigger/BPI_EventAction.Action`
  (params (`Action Type` :type "/Game/Kurai_Workspace/BlueprintTrigger/E_ActionType Enum" :default "NewEnumerator1") (msg :type String))
  (bind _returnvalue (`self.K2_GetActorLocation`))
  (bind _alien_ref (`self.Alien Ref`))
  (bind _alien_ref_2 (`self.Alien Ref`))
  (if (`|EnumEquality` `Action Type` "NewEnumerator4")
    (`KismetSystemLibrary.Delay` 2.0)
    (`self.Deactivate Entity`)
    (bind _returnvalue_2 (`NiagaraFunctionLibrary.SpawnSystemAtLocation` (`self.Niagara Mutaforma VFX`) _returnvalue))
    (`GameplayStatics.PlaySoundAtLocation` "/Game/Audio/trasformazione1.trasformazione1" _returnvalue (struct) 0.7 1.0 0.0 null null null null)
    (`KismetSystemLibrary.Delay` 5.0)
    (`ActorComponent.Deactivate` _returnvalue_2)
    (`self.Death`)
    (`self.Set Spawn Position` _alien_ref (+ (`self.K2_GetActorLocation`) (0.0 0.0 60.0)))
    (`self.Spawn` _alien_ref false "Player")
    (`self.Deactivate Entity` _alien_ref)
    (`|ExecutionSequence`
      (:`then_0`
        (bind (_direction _scale) (`Timeline|Scale Monster` :`NewTime` (`KismetStringLibrary.Conv_StringToDouble` msg) :!via `SetNewTime` :!label _label)
          (:`Update`
            (`SceneComponent.SetRelativeScale3D` (`Character.Mesh` (`self.Alien Ref`)) (`KismetMathLibrary.Conv_DoubleToVector` _scale)))
          (:`Finished`
            (`NavMovementComponent.StopActiveMovement` (`Character.CharacterMovement` _alien_ref_2))
            (bind _notifyname (`|PlayMontage` (`Character.Mesh` _alien_ref_2) "/Game/Test3DEnvironment/Characters/Alieno/Animazioni/AM_AlienScream.AM_AlienScream")
              (:`OnCompleted`
                (`self.Spawn` (`self.Alien Ref`) true "Player"))
              (:`OnNotifyBegin`
                (switch `name` _notifyname
                  (:`Scream`
                    (`GameplayStatics.PlaySoundAtLocation` "/Game/Audio/pollomostro.pollomostro" (`self.K2_GetActorLocation`) (struct) 4.0 1.0 0.0 null null null null))))))))
      (:`then_1`
        (goto _label)))
    (else
      (`parent.Action` `Action Type` msg))))

(fn `UserConstructionScript`
  (`parent.UserConstructionScript`))