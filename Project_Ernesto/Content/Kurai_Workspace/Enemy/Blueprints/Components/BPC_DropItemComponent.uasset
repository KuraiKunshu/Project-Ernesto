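; Enemy actor component that drops existing item actors at its owner's position.
; BeginPlay caches the owner, and the DropItems event loops over the valid actors passed in, acting only when ShowItems is true.
; Each item is unhidden and moved to the owner's X and Y with world Z fixed at zero.
; Items implementing IInteractable then have their interactability enabled.
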(event `self.ReceiveBeginPlay`
  ;[0 0 0] BeginPlay
  (set `self.OwnerRef` (`self.GetOwner`)))

(event `DropItems`
  (params (`Drop Items ` :type "Array of Actor Object Reference") (ShowItems :type Boolean))
  (bind (_returnvalue_x _returnvalue_y) (`KismetMathLibrary.BreakVector` (`Actor.K2_GetActorLocation` (`self.OwnerRef`))))
  ;[0 0 0] Drop Items
  (for _array_element `Drop Items `
    (`/Engine/EditorBlueprintResources/StandardMacros.IsValid` _array_element
      (:`Is Valid`
        (if ShowItems
          (`Actor.SetActorHiddenInGame` _array_element false)
          (`Actor.K2_SetActorLocation` _array_element (`KismetMathLibrary.MakeVector` _returnvalue_x _returnvalue_y) false false)
          (if (`KismetSystemLibrary.DoesImplementInterface` _array_element "/Game/Kurai_Workspace/Enemy/Blueprints/Interfaces/IInteractable.IInteractable_C")
            (bind _asiinteractable (cast `/Game/Kurai_Workspace/Enemy/Blueprints/Interfaces/IInteractable` _array_element))
            (`/Game/Kurai_Workspace/Enemy/Blueprints/Interfaces/IInteractable.SetInteractability` _asiinteractable ShowItems)))))))