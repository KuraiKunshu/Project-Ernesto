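; Health component, filed under Enemy, that tracks current HP and a shield for its owner.
; Initialize fills HP and zeroes the shield, ResetHealth refills HP only, and AddHp clamps the result between zero and max.
; TakeDamage drains the shield first, carrying overflow into HP.
; It reports whether HP stays above zero only when HP is hit; the branch where the shield absorbs everything has no explicit return.
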(event `self.ReceiveBeginPlay`)

(event `Initialize`
  (set `self.Current Hp` (`self.Max Hp`))
  (set `self.Shield` 0.0))

(event `Reset Health`
  (set `self.Current Hp` (`self.Max Hp`)))

(event `Add Hp`
  (params (`Hp Amount` :type "Float (double-precision)"))
  (bind _output_get (set `self.Current Hp` (+ (`self.Current Hp`) `Hp Amount`)))
  (set `self.Current Hp` (`KismetMathLibrary.FClamp` _output_get 0.0 (`self.Max Hp`))))

(fn `Take Damage`
  (params (Damage :type "Float (double-precision)") (`Damage Type` :type "DamageType Object Reference") (`Instigated By` :type "Controller Object Reference") (`Damage Causer` :type "Actor Object Reference"))
  (returns (IsAlive :type Boolean))
  (if (> (`self.Shield`) 0.0)
    (bind _output_get (set `self.Shield` (- (`self.Shield`) Damage)))
    (if (< _output_get 0.0)
      (set `self.Current Hp` (+ (`self.Current Hp`) (`self.Shield`)))
      (set `self.Shield` 0.0)
      (return (> (`self.Current Hp`) 0.0)))
    (else
      (set `self.Current Hp` (- (`self.Current Hp`) Damage))
      (return (> (`self.Current Hp`) 0.0)))))