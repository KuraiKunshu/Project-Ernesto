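; Base Blueprint for brawler enemies that deal melee damage through a sphere collider attached to mesh sockets.
; On attack, it looks up the montage in a map to snap the collider to that bone and set its radius, then calls the parent attack.
; Attack begin and end events toggle the damage and body colliders oppositely.
; BeginPlay starts in the non-attacking state on a default socket, and overlaps apply damage.
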(event `self.ReceiveBeginPlay`
  (`parent.ReceiveBeginPlay`)
  (`self.Attack End Behavior`)
  (`self.Attach Default Collider`))

(event `self.Damage Collider.OnComponentBeginOverlap`
  (params (OverlappedComponent :type "PrimitiveComponent Object Reference") (OtherActor :type "Actor Object Reference") (OtherComp :type "PrimitiveComponent Object Reference") (OtherBodyIndex :type Integer) (bFromSweep :type Boolean) (SweepResult :type "HitResult Structure (by ref)"))
  ;[0.2078 0.2078 0.2078] Attack
  (`GameplayStatics.ApplyDamage` OtherActor (`self.Attack Damage`) (`self.GetController` self) self))

(event `self.Attack Begin Behavior`
  ;[0.2078 0.2078 0.2078] Attack
  (`self.Set Enemy Attack Collider` true)
  (`self.Set Body Collider` false))

(event `self.Attack End Behavior`
  ;[0.2078 0.2078 0.2078] Attack
  (`self.Set Enemy Attack Collider` false)
  (`self.Set Body Collider` true))

(event `self.Attack`
  (params (`Attack Animation Montage` :type "AnimMontage Object Reference"))
  (bind (_value _returnvalue) (`BlueprintMapLibrary.Map_Find` (`self.Damage Collider Attacks Socket`) `Attack Animation Montage`))
  ;[0.2078 0.2078 0.2078] Attack
  (if _returnvalue
    (`self.Attach Collider` _value))
  (`parent.Attack` `Attack Animation Montage`))

(fn `Attach Collider`
  (params (`Attack Animation Collider` :type "/Game/Kurai_Workspace/Enemy/Blueprints/S_AttackSocket Structure"))
  (bind _returnvalue (`SceneComponent.K2_AttachToComponent` (`self.Damage Collider`) (`self.Mesh`) `Attack Animation Collider_BoneToAttach_7_F201B0F842E96742F9C81891053F5D9B` "SnapToTarget" "SnapToTarget" "SnapToTarget" true))
  (if _returnvalue
    (`SphereComponent.SetSphereRadius` (`self.Damage Collider`) `Attack Animation Collider_EnemyColliderSphereRadius_11_F9E75D554D90FD70F6803B8ED85D49B2` true)
    (else
      (`KismetSystemLibrary.PrintString` "Couldnt attach damage collider to socket" true true (struct :`R` 1.0 :`G` 0.648287 :`A` 1.0)))))

(fn `Attach Collider With Animation`
  (params (`Attack Animation` :type "AnimMontage Object Reference (by ref)"))
  (bind (_value _returnvalue) (`BlueprintMapLibrary.Map_Find` (`self.Damage Collider Attacks Socket`) `Attack Animation`))
  (if _returnvalue
    (`self.Attach Default Collider`)
    (else
      (`self.Attach Collider` _value))))

(fn `Attach Default Collider`
  (`self.Attach Collider` (make `/Game/Kurai_Workspace/Enemy/Blueprints/S_AttackSocket` (`self.Default Socket Name`) (`self.Default Collider Radius`))))

(fn `Set Enemy Attack Collider`
  (params (`bEnable?` :type Boolean))
  (`self.Set Collider` `bEnable?` (`self.Damage Collider`)))

(fn `UserConstructionScript`
  (`parent.UserConstructionScript`))