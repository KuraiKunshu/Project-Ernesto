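; Alien enemy Blueprint that overrides its parent's Action event to add a scream-and-retreat behavior.
; One action type plays the AM_AlienScream montage, and all other types pass through to the parent.
; Montage notifies drive the sequence: Scream plays a loud sound at the alien's location, while Walk Away disables fighting and moves it to the last entry in its target position list.
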(event `/Game/Kurai_Workspace/BlueprintTrigger/BPI_EventAction.Action`
  (params (`Action Type` :type "/Game/Kurai_Workspace/BlueprintTrigger/E_ActionType Enum" :default "NewEnumerator1") (msg :type String))
  (bind _target_position_list (`self.Target Position List`))
  (if (`|EnumEquality` `Action Type` "NewEnumerator4")
    (bind _notifyname (`|PlayMontage` (`self.Mesh`) "/Game/Test3DEnvironment/Characters/Alieno/Animazioni/AM_AlienScream.AM_AlienScream")
      (:`OnNotifyBegin`
        (switch `name` _notifyname
          (:`Walk Away`
            (`self.Set Can Fight` false)
            (`self.Move To Position` (`|GetArrayItem` _target_position_list (`KismetArrayLibrary.Array_LastIndex` _target_position_list))))
          (:`Scream`
            (`GameplayStatics.PlaySoundAtLocation` "/Game/Audio/pollomostro.pollomostro" (`self.K2_GetActorLocation`) (struct) 4.0 1.0 0.0 null null null null)))))
    (else
      (`parent.Action` `Action Type` msg))))

(fn `UserConstructionScript`
  (`parent.UserConstructionScript`))