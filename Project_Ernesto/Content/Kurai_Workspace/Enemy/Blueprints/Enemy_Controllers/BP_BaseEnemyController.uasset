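; Base enemy AI controller that reacts to AI Perception sight updates to track or drop a fightable target.
; Seeing the target records it and starts a looping attack-range check; losing sight stops that check and starts a delayed reset of the perceived actor.
; A target that fails the fight check clears both timers, resets perception state and halts movement.
; SetSightEnable toggles the sight sense.
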(event `self.ReceivePossess`
  (params (PossessedPawn :type "Pawn Object Reference"))
  (`parent.ReceivePossess` PossessedPawn))

(event `self.AIPerception.OnTargetPerceptionUpdated`
  (params (Actor :type "Actor Object Reference") (Stimulus :type "AIStimulus Structure"))
  (bind (_has_tag _can_fight___has_tag _can_fight) (`self.Can Fight Target` Actor))
  (if _can_fight
    (bind _returnvalue (`AIPerceptionSystem.GetSenseClassForStimulus` Stimulus))
    (if (== _returnvalue "/Script/AIModule.AISense_Sight")
      (if (`.bSuccessfullySensed` (break `AIStimulus` Stimulus))
        (`KismetSystemLibrary.K2_ClearAndInvalidateTimerHandle` (`self.Line Of Sight Timer`))
        (`self.Set Percived Actor` true (`self.Main Target`))
        (bind _returnvalue_2 (`KismetSystemLibrary.K2_SetTimer` null "Check Attack Range" (`self.Check Attack Range Time`) true false 0.0 0.1))
        (set `self.Check Attack Range Timer` _returnvalue_2)
        (else
          (bind _returnvalue_3 (`KismetSystemLibrary.K2_SetTimer` null "Reset Percived Actor" (`self.Line Of Sight Time`) false false 0.0 0.1))
          (set `self.Line Of Sight Timer` _returnvalue_3)
          (`KismetSystemLibrary.K2_ClearAndInvalidateTimerHandle` (`self.Check Attack Range Timer`)))))
    (else
      (`KismetSystemLibrary.K2_ClearAndInvalidateTimerHandle` (`self.Line Of Sight Timer`))
      (`KismetSystemLibrary.K2_ClearAndInvalidateTimerHandle` (`self.Check Attack Range Timer`))
      (`self.Reset Percived Actor`)
      (`self.StopMovement`)
      (`NavMovementComponent.StopActiveMovement` (`Character.CharacterMovement` (`self.Possessed Enemy`))))))

(event `self.Forget All Entity Perceived`)

(fn `Set Sight Enable`
  (params (bEnable :type Boolean))
  (`AIPerceptionComponent.SetSenseEnabled` (`self.AIPerception`) "/Script/AIModule.AISense_Sight" bEnable))

(fn `UserConstructionScript`)