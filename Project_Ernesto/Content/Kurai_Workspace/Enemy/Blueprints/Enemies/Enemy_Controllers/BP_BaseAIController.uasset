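; Base AI controller for enemies that caches the possessed BP_BaseEnemy and its attack distance, and manages target and combat state.
; It wraps Blackboard access in validity-checked helpers for can-attack, line-of-sight and target reference, printing on failure.
; Targets are matched by actor tag (default Player), and a distance check to the main target sets the can-attack flag.
; Helpers start and stop the behavior tree, while init, de-init and forget-perceived events are empty stubs.
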(event `Init Controller`)

(event `De-Init Controller`)

(event `Forget All Entity Perceived`)

(event `self.ReceivePossess`
  (params (PossessedPawn :type "Pawn Object Reference"))
  (bind _asbp_base_enemy (cast `/Game/Kurai_Workspace/Enemy/Blueprints/Enemies/BP_BaseEnemy` PossessedPawn))
  (set `self.Possessed Enemy` _asbp_base_enemy)
  (set `self.Attack Distance` (`/Game/Kurai_Workspace/Enemy/Blueprints/Enemies/BP_BaseEnemy.Attack Distance` _asbp_base_enemy)))

(event `Init Controller (E O)`
  ;[1 1 1] Editor Only
  (`self.Init Controller`))

(event `Check Attack Range`
  (`/Engine/EditorBlueprintResources/StandardMacros.IsValid` (`self.Main Target`)
    (:`Is Valid`
      (if (<= (`KismetMathLibrary.Vector_Distance` (`self.K2_GetActorLocation` (`self.Possessed Enemy`)) (`self.K2_GetActorLocation` (`self.Main Target`))) (`self.Attack Distance`))
        (`self.Set Can Attack` true)
        (else
          (`self.Set Can Attack` false))))
    (:`Is Not Valid`
      (`KismetSystemLibrary.PrintString` (`KismetStringLibrary.Concat_StrStr` "Actor Percived Null for Tag: " (`KismetStringLibrary.Conv_NameToString` (`self.Current Target Tag`)))))))

(event `De-Init Controller (E O)`
  ;[1 1 1] Editor Only
  (`self.De-Init Controller`))

(event `Reset Percived Actor`
  (`self.Set Percived Actor` false))

(fn `Can Fight Target`
  (params (`Target Percived` :type "Actor Object Reference"))
  (returns (`Has Tag` :type Boolean) (`Can Fight & Has Tag` :type Boolean) (`Can Fight` :type Boolean))
  (bind _returnvalue (`self.ActorHasTag` `Target Percived` (`self.Current Target Tag`)))
  (bind _can_fight (`/Game/Kurai_Workspace/Enemy/Blueprints/Enemies/BP_BaseEnemy.Can Fight` (`self.Possessed Enemy`)))
  (if _returnvalue
    (set `self.Main Target` `Target Percived`))
  (return _returnvalue (and _returnvalue _can_fight) _can_fight))

(fn `Get BlackBoard Bool`
  (params (KeyName :type "Name (by ref)"))
  (returns (ReturnValue :type Boolean))
  (`/Engine/EditorBlueprintResources/StandardMacros.IsValid` (`self.Blackboard`)
    (:`Is Valid`
      (return (`BlackboardComponent.GetValueAsBool` (`self.Blackboard`) KeyName)))
    (:`Is Not Valid`
      (`KismetSystemLibrary.PrintString` (`KismetStringLibrary.Concat_StrStr` "Blackboard NOT Valid For \"" (`KismetStringLibrary.Conv_NameToString` KeyName) "\" Call") true true (struct :`R` 1.0 :`G` 0.05137 :`A` 1.0)))))

(fn `Get BlackBoard Object`
  (params (KeyName :type "Name (by ref)"))
  (returns (ReturnValue :type "Object Object Reference"))
  (`/Engine/EditorBlueprintResources/StandardMacros.IsValid` (`self.Blackboard`)
    (:`Is Valid`
      (return (`BlackboardComponent.GetValueAsObject` (`self.Blackboard`) KeyName)))
    (:`Is Not Valid`
      (`KismetSystemLibrary.PrintString` (`KismetStringLibrary.Concat_StrStr` "Blackboard NOT Valid For \"" (`KismetStringLibrary.Conv_NameToString` KeyName) "\" Call") true true (struct :`R` 1.0 :`G` 0.05137 :`A` 1.0)))))

(fn `Get Can Attack`
  (returns (`Can Attack` :type Boolean))
  (bind _returnvalue (`self.Get BlackBoard Bool` (`self.Can Attack Key Name`)))
  (return _returnvalue))

(fn `Get Has Line Of Sight`
  (returns (Return :type Boolean))
  (bind _returnvalue (`self.Get BlackBoard Bool` (`self.Has Line Of Sight Key Name`)))
  (return _returnvalue))

(fn `Get Target Percived`
  (returns (`Target Ref` :type "Actor Object Reference") (`Is Actor` :type Boolean))
  (bind _returnvalue (`self.Get BlackBoard Object` (`self.Target Ref Key Name`)))
  (bind _asactor (cast `Actor` _returnvalue)
    (:`then`
      (return _asactor true))
    (:`CastFailed`
      (return null false))))

(fn `Set BlackBoard Bool`
  (params (KeyName :type "Name (by ref)") (BoolValue :type Boolean))
  (`/Engine/EditorBlueprintResources/StandardMacros.IsValid` (`self.Blackboard`)
    (:`Is Valid`
      (`BlackboardComponent.SetValueAsBool` (`self.Blackboard`) KeyName BoolValue))
    (:`Is Not Valid`
      (`KismetSystemLibrary.PrintString` (`KismetStringLibrary.Concat_StrStr` "Blackboard NOT Valid For Set \"" (`KismetStringLibrary.Conv_NameToString` KeyName) "\" To " (`KismetStringLibrary.Conv_BoolToString` BoolValue)) true true (struct :`R` 1.0 :`G` 0.05137 :`A` 1.0)))))

(fn `Set BlackBoard Object`
  (params (KeyName :type "Name (by ref)") (ObjectValue :type "Object Object Reference"))
  (`/Engine/EditorBlueprintResources/StandardMacros.IsValid` (`self.Blackboard`)
    (:`Is Valid`
      (`BlackboardComponent.SetValueAsObject` (`self.Blackboard`) KeyName ObjectValue))
    (:`Is Not Valid`
      (`KismetSystemLibrary.PrintString` (`KismetStringLibrary.Concat_StrStr` "Blackboard NOT Valid For Set \"" (`KismetStringLibrary.Conv_NameToString` KeyName) "\" To " (`KismetSystemLibrary.GetDisplayName` ObjectValue)) true true (struct :`R` 1.0 :`G` 0.05137 :`A` 1.0)))))

(fn `Set Can Attack`
  (params (BoolValue :type Boolean))
  (`self.Set BlackBoard Bool` (`self.Can Attack Key Name`) BoolValue))

(fn `Set Has Line Of Sight`
  (params (BoolValue :type Boolean))
  (`self.Set BlackBoard Bool` (`self.Has Line Of Sight Key Name`) BoolValue))

(fn `Set Percived Actor`
  (params (HasLineOfSight :type Boolean) (`Actor Percived` :type "Actor Object Reference"))
  (`self.Set Has Line Of Sight` HasLineOfSight)
  (`self.Set Target Percived` `Actor Percived`))

(fn `Set Target Percived`
  (params (ObjectValue :type "Actor Object Reference"))
  (`self.Set BlackBoard Object` (`self.Target Ref Key Name`) ObjectValue))

(fn `Set Target Tag`
  (params (`Target Tag` :type Name))
  (if (== `Target Tag` "None")
    (set `self.Current Target Tag` "Player")
    (else
      (set `self.Current Target Tag` `Target Tag`)))
  (return))

(fn `Start Logic`
  (params (BTAsset :type "BehaviorTree Object Reference"))
  (`/Engine/EditorBlueprintResources/StandardMacros.IsValid` BTAsset
    (:`Is Valid`
      (bind _returnvalue (`self.RunBehaviorTree` BTAsset))
      (if _returnvalue
        (`BrainComponent.StartLogic` (`self.BrainComponent`))
        (else
          (`KismetSystemLibrary.PrintString` "Coudnt Run Tree" true true (struct :`R` 1.0 :`G` 0.015156 :`A` 1.0) 10.0))))
    (:`Is Not Valid`
      (`KismetSystemLibrary.PrintString` "BT NOT VALID"))))

(fn `Stop Logic`
  (bind _braincomponent (`self.BrainComponent`))
  (`/Engine/EditorBlueprintResources/StandardMacros.IsValid` _braincomponent
    (:`Is Valid`
      (`BrainComponent.StopLogic` _braincomponent ""))
    (:`Is Not Valid`
      (`KismetSystemLibrary.PrintString` "Brain Component Not Valid For Stop" true true (struct :`R` 1.0 :`G` 0.071324 :`A` 1.0)))))

(fn `UserConstructionScript`)