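; Base enemy character with health, patrol, montage attacks, stagger and death, driven by a behavior tree on BP_BaseAIController.
; Activation and deactivation toggle AI logic and linked anim layers; enemies start hidden without collision, and Spawn resets and reveals them for reuse.
; Damage goes through BPCHealthModule, targeting the player and triggering a timed stagger or death, which hides rather than destroys the enemy.
; Random attack montages route notifies to empty behavior hooks.
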(event `Deabilitate (EO)`
  ;[1 1 1] Only On Editor
  (`self.Deactivate Enemy`))

(event `self.ReceiveBeginPlay`
  (`|ExecutionSequence`
    (:`then_0`
      ;[0.2086 0.2086 0.2086] Base Set up for Animation
      (set `self.Animation BP Class` (`SkeletalMeshComponent.AnimClass` (`self.Mesh`)))
      ;[0.3365 0.3365 0.3365] Set Material Reference
      (`self.Set Material`))
    (:`then_1`
      ;[0.2086 0.2086 0.2086] Set Patrol World Position
      (for _array_element (`self.Target List`)
        (`KismetArrayLibrary.Array_Add` (`self.Target Position List`) (`self.K2_GetActorLocation` _array_element)))
      ;;[1 1 1] Add spawn location to target list
      (`KismetArrayLibrary.Array_Add` (`self.Target Position List`) (`self.K2_GetActorLocation`)))
    (:`then_3`
      ;[0.2086 0.2086 0.2086] Without it, they Despawn
      (add `self.OnEnemyDeath` (delegate `Death`))
      ;[0.2078 0.2078 0.2078] Health System
      (`self.Set Enemy Body Collider` false :!label _label)
      (`SceneComponent.SetHiddenInGame` (`self.Mesh`) true false))))

(event `Abilitate (EO)`
  ;[1 1 1] Only On Editor
  (`self.Activate Enemy` "Player"))

(event `Set Can Fight (EO)`
  ;[1 1 1] Only On Editor
  (`self.Set Can Fight` (not (`self.Can Fight`))))

(event `Death (EO)`
  ;[1 1 1] Only On Editor
  (`self.Death`))

(event `Death`
  ;[0.2078 0.2078 0.2078] Health System
  (set `self.Is Dead` true)
  (`self.Deactivate Enemy`)
  (`KismetSystemLibrary.Delay` (`self.Death animation time`))
  (goto _label))

(event `Spawn (EO)`
  ;[1 1 1] Only On Editor
  (`self.Spawn` false))

(event `self.ReceiveAnyDamage`
  (params (Damage :type "Float (single-precision)") (DamageType :type "DamageType Object Reference") (InstigatedBy :type "Controller Object Reference") (DamageCauser :type "Actor Object Reference"))
  ;[0.2078 0.2078 0.2078] Health System
  (bind _isalive (`/Game/Kurai_Workspace/Enemy/Blueprints/Components/BPC_HealthModule.Take Damage` (`self.BPC_HealthModule`) Damage DamageType InstigatedBy DamageCauser))
  (`self.Set Target` "Player")
  (if _isalive
    (`self.Start Stagger` true)
    (`self.Stagger_Anim`)
    (else
      (`self.OnEnemyDeath`)))
  (`self.OnAnimationEnded`))

(event `Random Attack`
  ;[0.2078 0.2078 0.2078] Attack
  (bind (_has_any_attack_animations _attack_animation) (`self.Get Random Animation`))
  (if _has_any_attack_animations
    (`self.Attack` _attack_animation)))

(event `Attack`
  (params (`Attack Animation Montage` :type "AnimMontage Object Reference"))
  ;[0.2078 0.2078 0.2078] Attack
  (bind _notifyname (`|PlayMontage` (`self.Mesh`) `Attack Animation Montage`)
    (:`OnCompleted`
      (`self.OnAnimationEnded`))
    (:`OnNotifyBegin`
      (switch `name` _notifyname
        (:`Begin Attack`
          (`self.Attack Begin Behavior`))
        (:`End Attack`
          (`self.Attack End Behavior`))
        (:`Special`
          (`self.Special Attack Behavior`))))))

(event `Attack Begin Behavior`
  ;[0.2078 0.2078 0.2078] Attack
)

(event `Attack End Behavior`
  ;[0.2078 0.2078 0.2078] Attack
)

(event `Special Attack Behavior`
  ;[0.2078 0.2078 0.2078] Attack
)

(event `Move To Path`
  (bind _target_position_list (`self.Target Position List`))
  ;[0.2086 0.2086 0.2086] Pathfinding
  (if (`self.Is Dead`)
    _
    (elif (> (`KismetArrayLibrary.Array_Length` _target_position_list) 0)
      (`|AIMoveTo` self (`NavigationSystemV1.K2_GetRandomReachablePointInRadius` (`|GetArrayItem` _target_position_list (`self.TargetIndex`)) (`self.Radius`) (`self.Nav Data`) null) null
        (:`OnSuccess`
          _)
        (:`OnFail`
          (`KismetSystemLibrary.PrintString` "NO Path Found" true true (struct :`R` 1.0 :`G` 0.524 :`A` 1.0))))
      (bind _result (`/Engine/EditorBlueprintResources/StandardMacros.IncrementInt` (`self.TargetIndex`))
        (:`  `
          (if (>= _result (`KismetArrayLibrary.Array_Length` (`self.Target Position List`)))
            (set `self.TargetIndex` 0)))))))

(event `Start Stagger`
  (params (bCanReturnToFight :type Boolean))
  ;[0.2086 0.2086 0.2086] Stagger
  (set `self.is Staggered` true)
  (`self.Deactivate Enemy`)
  (`KismetSystemLibrary.RetriggerableDelay` (`self.Stagger Duration`))
  (`self.Activate Enemy` "Player")
  (`self.Set Can Fight` bCanReturnToFight)
  (set `self.is Staggered` false))

(event `self.ReceivePossessed`
  (params (NewController :type "Controller Object Reference"))
  ;[0.2086 0.2086 0.2086] Check Controller
  (bind _asbp_base_aicontroller (cast `/Game/Kurai_Workspace/Enemy/Blueprints/Enemies/Enemy_Controllers/BP_BaseAIController` NewController)
    (:`then`
      (set `self.Enemy Controller` _asbp_base_aicontroller))
    (:`CastFailed`
      (`KismetSystemLibrary.PrintString` "azz, controller sbagliato" true true (struct :`R` 1.0 :`G` 0.266226 :`A` 1.0) 10.0))))

(event `Stagger_Anim`)

(fn `Activate Enemy`
  (params (TargetTag :type Name))
  (`SkeletalMeshComponent.LinkAnimClassLayers` (`self.Mesh`) (`self.Animation BP Class`))
  (`/Game/Kurai_Workspace/Enemy/Blueprints/Enemies/Enemy_Controllers/BP_BaseEnemyController.Set Target Tag` (`self.Enemy Controller`) TargetTag)
  (`/Game/Kurai_Workspace/Enemy/Blueprints/Enemies/Enemy_Controllers/BP_BaseAIController.Start Logic` (`self.Enemy Controller`) (`self.Behavior Tree`))
  (`/Game/Kurai_Workspace/Enemy/Blueprints/Enemies/Enemy_Controllers/BP_BaseAIController.Init Controller` (`self.Enemy Controller`)))

(fn `Change Aggro Distance`
  (params (`New Aggro Distance` :type "Float (double-precision)"))
  (set `self.Aggro Distance` `New Aggro Distance`))

(fn `Change Stagger Material`
  (locals (StaggerMaterial :type "MaterialInterface Object Reference" :default "/Script/Engine.MaterialInstanceConstant'/Game/MonsterForSurvivalGame/Material/MI_HitEnemy.MI_HitEnemy'"))
  (`PrimitiveComponent.SetMaterial` (`self.Mesh`) 0 (`local.StaggerMaterial`))
  (return))

(fn `Deactivate Enemy`
  (`NavMovementComponent.StopActiveMovement` (`self.CharacterMovement`))
  (`SkeletalMeshComponent.UnlinkAnimClassLayers` (`self.Mesh`) (`self.Animation BP Class`))
  (`self.Set Sight Enable` false)
  (`/Game/Kurai_Workspace/Enemy/Blueprints/Enemies/Enemy_Controllers/BP_BaseAIController.Stop Logic` (`self.Enemy Controller`))
  (`/Game/Kurai_Workspace/Enemy/Blueprints/Enemies/Enemy_Controllers/BP_BaseAIController.De-Init Controller` (`self.Enemy Controller`))
  (set `self.Can Fight` false))

(fn `Deal Damage`
  (params (`Damaged Actor` :type "Actor Object Reference"))
  (if (`self.ActorHasTag` `Damaged Actor` "Player")
    (`GameplayStatics.ApplyDamage` `Damaged Actor` (`self.Attack Damage`) null self)))

(fn `Get Random Animation`
  (returns (`Has Any Attack Animations` :type Boolean) (`Attack Animation` :type "AnimMontage Object Reference"))
  (bind _attack_animations (`self.Attack Animations`))
  (return (> (`KismetArrayLibrary.Array_Length` _attack_animations) 0) (`KismetArrayLibrary.Array_Random` _attack_animations)))

(fn `Reset Material`
  (`PrimitiveComponent.SetMaterial` (`self.Mesh`) 0 (`self.MaterialRef`)))

(fn `Set Can Fight`
  (params (`Can Fight` :type Boolean))
  (if (!= `Can Fight` (`self.Can Fight`))
    (set `self.Can Fight` `Can Fight`)
    (`self.Set Sight Enable` `Can Fight`)
    (`/Game/Kurai_Workspace/Enemy/Blueprints/Enemies/Enemy_Controllers/BP_BaseAIController.Forget All Entity Perceived` (`self.Enemy Controller`))))

(fn `Set Enemy Body Collider`
  (params (`bEnable?` :type Boolean))
  (`self.Set Enemy Collider` `bEnable?` (`self.CapsuleComponent`)))

(fn `Set Enemy Collider`
  (params (`bEnable?` :type Boolean) (Collider :type "PrimitiveComponent Object Reference"))
  (if `bEnable?`
    (`PrimitiveComponent.SetCollisionEnabled` Collider "QueryAndPhysics")
    (else
      (`PrimitiveComponent.SetCollisionEnabled` Collider "NoCollision")))
  (`PrimitiveComponent.SetEnableGravity` Collider `bEnable?`)
  (return))

(fn `Set Material`
  (set `self.MaterialRef` (`PrimitiveComponent.GetMaterial` (`self.Mesh`) 0)))

(fn `Set Sight Enable`
  (params (InputPin :type Boolean))
  (bind _asbp_base_enemy_controller (cast `/Game/Kurai_Workspace/Enemy/Blueprints/Enemies/Enemy_Controllers/BP_BaseEnemyController` (`self.Enemy Controller`)))
  (`/Game/Kurai_Workspace/Enemy/Blueprints/Enemies/Enemy_Controllers/BP_BaseEnemyController.Set Sight Enable` _asbp_base_enemy_controller InputPin))

(fn `Set Spawn Position`
  (params (`New Spawn Position` :type "Vector Structure"))
  (bind _target_position_list (`self.Target Position List`))
  (`KismetArrayLibrary.Array_Set` _target_position_list (`KismetArrayLibrary.Array_LastIndex` _target_position_list) `New Spawn Position`)
  (return))

(fn `Set Target`
  (params (Target :type Name))
  (`/Game/Kurai_Workspace/Enemy/Blueprints/Enemies/Enemy_Controllers/BP_BaseEnemyController.Set Target Tag` (`self.Enemy Controller`) Target)
  (return))

(fn `Set Walk Max Speed`
  (params (`Max Speed` :type "Float (double-precision)"))
  (set `CharacterMovementComponent.MaxWalkSpeed` `Max Speed` (`self.CharacterMovement`)))

(fn `Spawn`
  (params (bCanFight :type Boolean) (TargetTag :type Name))
  (bind _target_position_list (`self.Target Position List`))
  (`/Game/Kurai_Workspace/Enemy/Blueprints/Components/BPC_HealthModule.Initialize` (`self.BPC_HealthModule`))
  (set `self.Is Dead` false)
  (`self.Activate Enemy` TargetTag)
  (`self.Set Enemy Body Collider` true)
  (`self.K2_SetActorLocation` (`|GetArrayItem` _target_position_list (`KismetArrayLibrary.Array_LastIndex` _target_position_list)) false true)
  (set `self.TargetIndex` 0)
  (`SceneComponent.SetHiddenInGame` (`self.Mesh`) false false)
  (`self.Set Can Fight` bCanFight)
  (`self.Set Sight Enable` bCanFight))

(fn `Spawn Controller Actor`
  (params (`Controller Class` :type "Controller Class Reference"))
  (bind _asbp_base_aicontroller (castclass `/Game/Kurai_Workspace/Enemy/Blueprints/Enemies/Enemy_Controllers/BP_BaseAIController` `Controller Class`))
  (bind _returnvalue (`|SpawnActorFromClass` _asbp_base_aicontroller (`self.GetTransform`) "AlwaysSpawn" "MultiplyWithRoot" null null))
  (`Controller.Possess` _returnvalue self)
  (`/Game/Kurai_Workspace/Enemy/Blueprints/Enemies/Enemy_Controllers/BP_BaseAIController.Start Logic` _returnvalue (`self.Behavior Tree`))
  (`/Game/Kurai_Workspace/Enemy/Blueprints/Enemies/Enemy_Controllers/BP_BaseAIController.Init Controller` _returnvalue))

(fn `Spawn Own Controller Actor`
  (`self.Spawn Controller Actor` (`self.AIControllerClass`)))

(fn `UserConstructionScript`)