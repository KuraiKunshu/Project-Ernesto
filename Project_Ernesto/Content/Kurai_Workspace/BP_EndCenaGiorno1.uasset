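; Scripted event actor that, going by its name, ends the day 1 dinner (cena) and leads into dialogue with BP_Zia_Giorno_1.
; Its Action event plays the BPW_ChangeScene transition widget in reverse, with timed delays around a sound at the player's location.
; It then forwards an action message to the Triggers actor, assigns that aunt's dialogue component to the first-person character and starts the interaction.
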(event `/Game/Kurai_Workspace/BlueprintTrigger/BPI_EventAction.Action`
  (params (`Action Type` :type "/Game/Kurai_Workspace/BlueprintTrigger/E_ActionType Enum" :default "NewEnumerator1") (msg :type String))
  (bind (_triggers_actor _triggers_actiontype _triggers_msg) (break `/Game/Kurai_Workspace/S_TriggerTemp` (`self.Triggers`)))
  (bind _returnvalue (`|CreateWidget` "/Game/Kurai_Workspace/BPW_ChangeScene.BPW_ChangeScene_C" (`GameplayStatics.GetPlayerController` 0)))
  (`UserWidget.AddToViewport` _returnvalue 0)
  (`/Game/Kurai_Workspace/BPW_ChangeScene.Play` _returnvalue "Reverse" 1.0)
  (`KismetSystemLibrary.Delay` 2.0)
  (`GameplayStatics.PlaySoundAtLocation` null (`self.K2_GetActorLocation` (`GameplayStatics.GetPlayerPawn` 0)) (struct) 1.0 1.0 0.0 null null null null)
  (`KismetSystemLibrary.Delay` 2.0)
  (message `/Game/Kurai_Workspace/BlueprintTrigger/BPI_EventAction.Action` _triggers_actor _triggers_actiontype _triggers_msg)
  (bind _asbp_zia_giorno_1 (cast `/Game/Kurai_Workspace/Enemy/Blueprints/BP_Zia_Giorno_1` _triggers_actor))
  (bind _asbp_first_person_character (cast `/Game/FirstPerson/Blueprints/BP_FirstPersonCharacter` (`GameplayStatics.GetPlayerPawn` 0)))
  (bind _output_get (set `/Game/FirstPerson/Blueprints/BP_FirstPersonCharacter.Dialogue Comp ref` (`/Game/Kurai_Workspace/Enemy/Blueprints/BP_BaseNPC.BPC_DialogueSystem` _asbp_zia_giorno_1) _asbp_first_person_character))
  (message `/Game/Kurai_Workspace/Enemy/Blueprints/Interfaces/IInteractable.Interact` _output_get))

(fn `UserConstructionScript`)