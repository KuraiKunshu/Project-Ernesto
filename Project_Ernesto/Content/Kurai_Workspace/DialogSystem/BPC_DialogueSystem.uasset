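; Actor component that runs data-table-driven dialogue for its owner, showing lines, player choices and follow-up dialogue.
; Each Interact shows the next line of the current DT_New_Dialogue row in a BPW_Dialogue widget, then offers any choices.
; Otherwise it closes the widget, queues the default next row, clears the first-person character's talking flag and sends the row's trigger action messages to target actors.
; A selected answer loads its linked row; missing rows print an error.
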(event `self.ReceiveBeginPlay`
  (set `self.Owner` (`self.GetOwner`)))

(event `/Game/Kurai_Workspace/Enemy/Blueprints/Interfaces/IInteractable.Interact`
  (bind _dialogue (`self.Get Dialogue`))
  (bind _has_trigger (`self.Get Triggers`))
  (bind (_out_row_dialoghi _out_row_thereisachoice _out_row_choices _out_row_prossimodefaultdialogo) (break `/Game/Kurai_Workspace/DialogSystem/S_DataTableStruct` (`self.Out Row`)))
  ;[1 1 1] Interact System
  (if (`self.Dialogue Finished`)
    _
    (elif (< (`self.Dialogue Index`) (`KismetArrayLibrary.Array_Length` _dialogue))
      (`self.Widget Ref`
        (:`then`
          _)
        (:`else`
          (`self.Set ViewPort`)))
      (`self.Set Text` (`|GetArrayItem` _dialogue (`self.Dialogue Index`)))
      (`/Engine/EditorBlueprintResources/StandardMacros.IncrementInt` (`self.Dialogue Index`))
      (elif (`self.Get There is a Choice`)
        (`self.Set Choice`)
        (set `self.Out Row` (make `/Game/Kurai_Workspace/DialogSystem/S_DataTableStruct` _out_row_dialoghi false _out_row_choices _out_row_prossimodefaultdialogo))
        (else
          (`self.Clear Viewport`)
          (if (!= (`self.Get Next Dialogue`) "None")
            (`self.Set Dialogue` (`self.Get Next Dialogue`)))
          (`self.Set Player Talking` false)
          (if (> (`KismetArrayLibrary.Array_Length` _has_trigger) 0)
            (for _array_element _has_trigger
              (message `/Game/Kurai_Workspace/BlueprintTrigger/BPI_EventAction.Action` (`|ConvertAsset` (`.Actor_8_DB63598C4010E8753F8E81B539739DFA` (break `/Game/Kurai_Workspace/DialogSystem/S_TriggerParameter` _array_element))) (break `/Game/Kurai_Workspace/DialogSystem/S_TriggerParameter` _array_element) (`.msg_5_4B1C3F28491F7F816097A88E34BE7D93` (break `/Game/Kurai_Workspace/DialogSystem/S_TriggerParameter` _array_element))))))))))

(event `Set Choice Dialogue`
  (params (Answer :type Text))
  ;[1 1 1] Interact System
  (for _array_element (`self.Get Choices`)
    (if (`KismetTextLibrary.EqualEqual_TextText` (break `/Game/Kurai_Workspace/DialogSystem/S_Choice` _array_element) Answer)
      (`self.Set Dialogue` (`.PROSSIMODIALOGO_5_9A7A06664FBE77FC0E54CDA9A36556D9` (break `/Game/Kurai_Workspace/DialogSystem/S_Choice` _array_element)))
      (break))))

(event `Set Dialogue`
  (params (`DT Row Name` :type Name))
  ;[1 1 1] Interact System
  (if (!= "None" `DT Row Name`)
    (bind _returnvalue (`|GetDataTableRow` "/Game/Kurai_Workspace/DialogSystem/DT_New_Dialogue.DT_New_Dialogue" `DT Row Name`)
      (:`then`
        (set `self.Out Row` _returnvalue)
        (set `self.Dialogue Index` 0)
        (set `self.Dialogue Finished` false)
        (bind _output_get (set `self.Row Name` `DT Row Name`))
        (`KismetSystemLibrary.PrintString` (`KismetStringLibrary.Concat_StrStr` "Dilogue " (`KismetStringLibrary.Conv_NameToString` _output_get) "Added")))
      (:`RowNotFound`
        (`KismetSystemLibrary.PrintString` (`KismetStringLibrary.Concat_StrStr` "NO ROW FOUND  " (`KismetStringLibrary.Conv_NameToString` `DT Row Name`) "(CONTROLLA CHE IL NOME DEL \"PROSSIMO DIALOGO\"  SIA GIUSTO, MAIUSCOLE INCLUSE)") true true (struct :`R` 1.0 :`G` 0.017282 :`A` 1.0) 20.0 :!label _label)))
    (else
      (goto _label))))

(fn `Clear Viewport`
  (`Widget.RemoveFromParent` (`self.Widget Ref`))
  (set `self.Widget Ref` null)
  (set `self.Dialogue Finished` true))

(fn `IsInteractable`
  (returns (Value :type Boolean))
  (return false))

(fn `Send Interaction`
  (params (`Action Type` :type "/Game/Kurai_Workspace/BlueprintTrigger/E_ActionType Enum" :default "NewEnumerator1") (msg :type String))
  (bind _owner (`self.Owner`))
  (`/Engine/EditorBlueprintResources/StandardMacros.IsValid` _owner
    (:`Is Valid`
      (message `/Game/Kurai_Workspace/BlueprintTrigger/BPI_EventAction.Action` _owner `Action Type` msg))))

(fn `Set Choice`
  (bind _widget_ref (`self.Widget Ref`))
  (set `/Game/Kurai_Workspace/DialogSystem/BPW_Dialogue.Npc Dialogue component ref` self _widget_ref)
  (`/Game/Kurai_Workspace/DialogSystem/BPW_Dialogue.Add Choice` _widget_ref (`self.Get Choices`)))

(fn `Set Player Talking`
  (params (`Is Talking` :type Boolean))
  (`self.Player Ref`
    (:`then`
      _)
    (:`else`
      (bind _asbp_first_person_character (cast `/Game/FirstPerson/Blueprints/BP_FirstPersonCharacter` (`GameplayStatics.GetPlayerPawn` 0)))
      (set `self.Player Ref` _asbp_first_person_character)))
  (set `/Game/FirstPerson/Blueprints/BP_FirstPersonCharacter.Is Talking` `Is Talking` (`self.Player Ref`)))

(fn `Set Text`
  (params (Text :type "/Game/Kurai_Workspace/DialogSystem/S_Dialogue Structure"))
  (set `TextBlock.Text` (`KismetTextLibrary.Conv_StringToText` (`|GetEnumeratorNameAsString` Text_TalkingEntity_2_06E58C2F450791BF3275C98FCA0C926E)) (`/Game/Kurai_Workspace/DialogSystem/BPW_Dialogue.TextTalkingName` (`self.Widget Ref`)))
  (set `TextBlock.Text` Text_Dialogue_5_33950CC5407A8FB433913890D2C5ED7C (`/Game/Kurai_Workspace/DialogSystem/BPW_Dialogue.TextBox` (`self.Widget Ref`))))

(fn `Set ViewPort`
  (bind _returnvalue (`|CreateWidget` "/Game/Kurai_Workspace/DialogSystem/BPW_Dialogue.BPW_Dialogue_C" (`GameplayStatics.GetPlayerController` 0)))
  (bind _output_get (set `self.Widget Ref` _returnvalue))
  (`UserWidget.AddToViewport` _output_get 0)
  (`self.Set Player Talking` true))