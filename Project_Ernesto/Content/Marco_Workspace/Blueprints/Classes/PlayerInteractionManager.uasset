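; Player interaction manager that handles looking at, picking up and using items through the E key and an on-screen tooltip.
; A camera-forward line trace finds the target: E sends it an interact message, or uses the held I_Item on it.
; HoldItem attaches an item to the player character and switches to held-item behaviour.
; A looping 0.2-second delay replaces Tick, refreshing the HUD tooltip from the target or held item.
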(event `self.ReceiveBeginPlay`
  (bind _returnvalue (`|CreateWidget` "/Game/Marco_Workspace/Blueprints/Classes/Widgets/Interaction_HUD.Interaction_HUD_C" (`GameplayStatics.GetPlayerController` 0)))
  (bind _output_get (set `self.HUD` _returnvalue))
  (`UserWidget.AddToViewport` _output_get 0)
  (`self.UpdateLoop`))

(event `Key|E`
  (params (Key :type "Key Structure"))
  (:`Pressed`
    (if (`self.IsHoldingItem`)
      (bind _asi_item (cast `/Game/Marco_Workspace/Blueprints/Interfaces/I_Item` (`self.HeldItem`)))
      (bind _outhit (`self.Raycast`))
      (`/Game/Marco_Workspace/Blueprints/Interfaces/I_Item.UseItem` _asi_item self _outhit)
      (else
        (bind _outhit_2 (`self.Raycast`))
        (message `/Game/Marco_Workspace/Blueprints/Interfaces/I_Interactable.Interact` (`.HitActor` (`GameplayStatics.BreakHitResult` _outhit_2)) self)))))

(event `UpdateLoop`
  (bind _hud (`self.HUD`))
  (if (`self.IsHoldingItem`) :!label _label
    (bind _outhit (`self.Raycast`))
    (message `/Game/Marco_Workspace/Blueprints/Interfaces/I_Item.ShowUseInfo` (`KismetSystemLibrary.Conv_InterfaceToObject` (`self.HeldItem`)) _hud _outhit)
    (else
      (bind _outhit_2 (`self.Raycast`))
      (message `/Game/Marco_Workspace/Blueprints/Interfaces/I_Interactable.ShowInfo` (`.HitActor` (`GameplayStatics.BreakHitResult` _outhit_2)) _hud)))
  (`KismetSystemLibrary.Delay` 0.2)
  (`/Game/Marco_Workspace/Blueprints/Classes/Widgets/Interaction_HUD.SetTooltipTextValue` _hud "")
  (goto _label))

(fn `Hold Item`
  (params (`New Item` :type "Actor Object Reference"))
  (bind _asi_item (cast `/Game/Marco_Workspace/Blueprints/Interfaces/I_Item` `New Item`))
  (bind _output_get (set `self.HeldItem` _asi_item))
  (`/Game/Marco_Workspace/Blueprints/Interfaces/I_Item.AttachToHolder` _output_get (`GameplayStatics.GetPlayerCharacter` 0))
  (set `self.IsHoldingItem` true))

(fn `Raycast`
  (returns (OutHit :type "HitResult Structure"))
  (bind _returnvalue (`GameplayStatics.GetPlayerCameraManager` 0))
  (bind _returnvalue_2 (`PlayerCameraManager.GetCameraLocation` _returnvalue))
  (bind _outhit (`KismetSystemLibrary.LineTraceSingle` _returnvalue_2 (+ _returnvalue_2 (* (`self.Raggio`) (`KismetMathLibrary.GetForwardVector` (`SceneComponent.K2_GetComponentRotation` (`PlayerCameraManager.TransformComponent` _returnvalue))))) "TraceTypeQuery1"))
  (return _outhit))