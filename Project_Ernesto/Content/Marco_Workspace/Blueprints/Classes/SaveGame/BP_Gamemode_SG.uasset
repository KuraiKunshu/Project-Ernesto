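; Game mode that saves and restores first-person player progress through a single save slot.
; On BeginPlay it loads the existing save or writes a fresh BP_SaveGame if none exists.
; Savegame reloads the slot object and stores the player's transform and flashlight flag, but always writes the storage key flag as false.
; LoadGame applies the saved transform and both item flags to the BP_FirstPersonCharacter.
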(event `self.ReceiveBeginPlay`
  (bind _returnvalue (`GameplayStatics.DoesSaveGameExist` "Save1"))
  (if _returnvalue
    (`self.Load Game`)
    (else
      (bind _returnvalue_2 (`GameplayStatics.CreateSaveGameObject` "/Game/Marco_Workspace/Blueprints/Classes/SaveGame/BP_SaveGame.BP_SaveGame_C"))
      (`GameplayStatics.SaveGameToSlot` _returnvalue_2 "Save1"))))

(event `Save game`
  (bind _returnvalue (`GameplayStatics.LoadGameFromSlot` "Save1"))
  (bind _asbp_save_game (cast `/Game/Marco_Workspace/Blueprints/Classes/SaveGame/BP_SaveGame` _returnvalue))
  (bind _asbp_first_person_character (cast `/Game/FirstPerson/Blueprints/BP_FirstPersonCharacter` (`GameplayStatics.GetPlayerCharacter` 0)))
  (set `/Game/Marco_Workspace/Blueprints/Classes/SaveGame/BP_SaveGame.HasFlashlight` (`/Game/FirstPerson/Blueprints/BP_FirstPersonCharacter.Has Flashlight` _asbp_first_person_character) _asbp_save_game)
  (set `/Game/Marco_Workspace/Blueprints/Classes/SaveGame/BP_SaveGame.HasStorageKey` false _asbp_save_game)
  (set `/Game/Marco_Workspace/Blueprints/Classes/SaveGame/BP_SaveGame.PlayerPosition` (`self.GetTransform` _asbp_first_person_character) _asbp_save_game)
  (`GameplayStatics.SaveGameToSlot` _asbp_save_game "Save1"))

(event `Load Game`
  (bind _returnvalue (`GameplayStatics.LoadGameFromSlot` "Save1"))
  (bind _asbp_save_game (cast `/Game/Marco_Workspace/Blueprints/Classes/SaveGame/BP_SaveGame` _returnvalue))
  (bind _asbp_first_person_character (cast `/Game/FirstPerson/Blueprints/BP_FirstPersonCharacter` (`GameplayStatics.GetPlayerCharacter` 0)))
  (`self.K2_SetActorTransform` _asbp_first_person_character (`/Game/Marco_Workspace/Blueprints/Classes/SaveGame/BP_SaveGame.PlayerPosition` _asbp_save_game) false false)
  (set `/Game/FirstPerson/Blueprints/BP_FirstPersonCharacter.Has Flashlight` (`/Game/Marco_Workspace/Blueprints/Classes/SaveGame/BP_SaveGame.HasFlashlight` _asbp_save_game) _asbp_first_person_character)
  (set `/Game/FirstPerson/Blueprints/BP_FirstPersonCharacter.HasStorageKey` (`/Game/Marco_Workspace/Blueprints/Classes/SaveGame/BP_SaveGame.HasStorageKey` _asbp_save_game) _asbp_first_person_character))

(fn `UserConstructionScript`)